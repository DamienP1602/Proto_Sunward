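; Bidirectional rope actor that restricts the physics movement of its rope endpoint to a plane.
; The construction script sets EndpointRope to a custom-plane constraint and passes its right vector to SetBoxCollisionLockVector as the lock vector.
; A note plans moving this to C++ using the actor's forward vector.
; The event graph is inactive, and a debug "Hello" log remains.
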(event EventBeginPlay
  (|CallParentFunction) ; This node is disabled and will not be called.\nDrag off pins to build functionality.
)

(event Collision|EventActorBeginOverlap
  (params (OtherActor :type Actor%20Object%20Reference))
  (|CallParentFunction OtherActor) ; This node is disabled and will not be called.\nDrag off pins to build functionality.
)

(event EventTick
  (params (DeltaSeconds :type Float%20%28single-precision%29))
  (|CallParentFunction DeltaSeconds) ; This node is disabled and will not be called.\nDrag off pins to build functionality.
)

(fn ConstructionScript
  (|CallParentFunction)
  (Utilities|String|LogString "Hello")
  ;[1 1 1] Do in c++, set the plane constraint mode to the forward vector of the actor in beginplay, or when the forward of the actor changes
  (Class|PrimitiveComponent|SetConstraintMode (Variables|Default|GetEndpointRope) "CustomPlane")
  (Class|DirectionnalRopeGPE|SetBoxCollisionLockVector (Variables|Default|GetEndpointRope) (Math|Vector|GetRightVector (Variables|Default|GetEndpointRope))))