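; BP_Displayable is an actor that switches between a static mesh with player-proximity shading and a MapCube.
; On BeginPlay it gives the mesh a dynamic material instance with in-range and out-of-range colors and a sphere radius.
; Until AsBeenSaw is set, Tick feeds the player pawn's location into that material.
; Enable shows only MapCube, Disable only the mesh, and DisableAll hides both, printing a debug string.
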(event EventBeginPlay
  (bind _staticmesh (Variables|Default|GetStaticMesh))
  (Utilities|FlowControl|Sequence
    (:then_0
      (bind _returnvalue (Rendering|Material|CreateDynamicMaterialInstance _staticmesh 0 "/Game/Greg/BP/Test.Test" "None" :!class /Script/Engine.PrimitiveComponent))
      (bind _output_get (Variables|Default|SetMI _returnvalue))
      (Rendering|Material|SetMaterial _staticmesh 0 _output_get))
    (:then_1
      (Rendering|Material|SetVectorParameterValue (Variables|Default|GetMI) "OutRangeColor" (Variables|Default|GetOutRangeColor) :!class /Script/Engine.MaterialInstanceDynamic)
      (Rendering|Material|SetVectorParameterValue (Variables|Default|GetMI) "InRangeColor" (Variables|Default|GetInRangeColor) :!class /Script/Engine.MaterialInstanceDynamic)
      (Rendering|Material|SetScalarParameterValue (Variables|Default|GetMI) "SphereRadius" (Variables|Default|GetmaxDistance) :!class /Script/Engine.MaterialInstanceDynamic))))

(event EventTick
  (params (DeltaSeconds :type Float%20%28single-precision%29))
  (bind _mi (Variables|Default|GetMI))
  (if (not (Variables|Default|GetasBeenSaw))
    (Rendering|Material|SetVectorParameterValue _mi "PlayerPos" (Math|Conversions|ToLinearColor(Vector) (Transformation|GetActorLocation (Pawn|GetControlledPawn (Game|GetPlayerController 0)))) :!class /Script/Engine.MaterialInstanceDynamic)
    (Rendering|Material|GetVectorParameterValue _mi "BaseColor" :!class /Script/Engine.MaterialInstanceDynamic)))

(fn ConstructionScript)

(fn Enable
  (Development|SetHiddeninGame (Variables|Default|GetStaticMesh) true false)
  (Development|SetHiddeninGame (Variables|Default|GetMapCube) false false))

(fn Disable
  (Development|SetHiddeninGame (Variables|Default|GetStaticMesh) false false)
  (Development|SetHiddeninGame (Variables|Default|GetMapCube) true false))

(fn DisableAll
  (Development|SetHiddeninGame (Variables|Default|GetStaticMesh) true false)
  (Development|SetHiddeninGame (Variables|Default|GetMapCube) true false)
  (Development|PrintString "Hello"))